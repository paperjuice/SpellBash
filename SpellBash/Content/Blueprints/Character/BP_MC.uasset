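; Player character that moves on input axes, turns to face the cursor and casts fireballs on left mouse release.
; Tick and click branch on authority, with remote paths forwarding through client events to server events for rotation and spawning.
; Rotation uses yaw toward player controller 0's cursor hit, read inside the server event.
; MCUtils clears the HasFired cooldown gate on Tick; PanCamera, uncalled here, eases the camera toward the mouse.
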(event `s_McRotateTowardsCursor`
  (params (Start :type "Vector Structure (by ref)"))
  ;[1 1 1] MC follows cursor position on 3D objects
  (`|ExecutionSequence`
    (:`then_0`
      (`self.K2_SetActorRotation` (`KismetMathLibrary.MakeRotator` 0.0 0.0 (.yaw (`KismetMathLibrary.FindLookAtRotation` Start (`.Location` (`GameplayStatics.BreakHitResult` (`PlayerController.GetHitResultUnderCursorByChannel` (`GameplayStatics.GetPlayerController` 0) "TraceTypeQuery3" false))))))))))

(event `self.ReceiveTick`
  (params (DeltaSeconds :type "Float (single-precision)"))
  (bind _returnvalue (`self.K2_GetActorLocation`))
  (`|ExecutionSequence`
    (:`then_0`
      (`/Engine/EditorBlueprintResources/ActorMacros.Switch Has Authority`
        (:`Authority`
          (`self.s_McRotateTowardsCursor` _returnvalue))
        (:`Remote`
          (`self.c_McRotateTowardsCursor` _returnvalue))))
    (:`then_1`
      (bind _returnvalue_2 (`MC_Utils.IsOnCooldown` (`self.MC_Utils`) (`self.HasFired`)))
      (set `self.HasFired` _returnvalue_2))))

(event `c_McRotateTowardsCursor`
  (params (Start :type "Vector Structure (by ref)"))
  ;[1 1 1] MC follows cursor position on 3D objects
  (`self.s_McRotateTowardsCursor` Start))

(event `self.ReceiveBeginPlay`
  (`|ExecutionSequence`
    (:`then_0`
      ;[1 1 1] Character Movement
      (set `CharacterMovementComponent.MaxWalkSpeed` (`self.MC_Speed`) (`self.CharacterMovement`)))
    (:`then_1`
      (set `MC_Utils.MaxCooldown` 0.4 (`self.MC_Utils`)))))

(event `InputAxis|Up_Down`
  (params (AxisValue :type "Float (single-precision)"))
  ;[1 1 1] Character Movement
  (`self.AddMovementInput` (`KismetMathLibrary.GetForwardVector` (`KismetMathLibrary.MakeRotator` 0.0 (.pitch (`self.GetControlRotation`)))) AxisValue))

(event `InputAxis|Left_Right`
  (params (AxisValue :type "Float (single-precision)"))
  ;[1 1 1] Character Movement
  (`self.AddMovementInput` (`KismetMathLibrary.GetRightVector` (`KismetMathLibrary.MakeRotator` 0.0 (.pitch (`self.GetControlRotation`)))) AxisValue))

(event `PanCamera`
  (params (DeltaTime :type "Float (double-precision)"))
  (bind _camera (`self.Camera`))
  (bind _worldlocation (`PlayerController.DeprojectMousePositionToWorld` (`GameplayStatics.GetPlayerController` 0)))
  (`SceneComponent.K2_SetWorldLocation` _camera (`KismetMathLibrary.MakeVector` (.x (`KismetMathLibrary.VInterpTo` (`SceneComponent.K2_GetComponentLocation` _camera) _worldlocation DeltaTime 10.0)) (.y (`KismetMathLibrary.VInterpTo` (`SceneComponent.K2_GetComponentLocation` _camera) _worldlocation DeltaTime 10.0)) (.z _worldlocation)) false false))

(event `ServerCastFireball`
  ;[1 1 1] Cast Fireball
  (if (not (`self.HasFired`))
    (set `self.HasFired` true)
    (`|SpawnActorFromClass` "/Game/Blueprints/Spells/BP_Fireball_01.BP_Fireball_01_C" (`KismetMathLibrary.MakeTransform` (.location (`SceneComponent.K2_GetComponentToWorld` (`self.SpawnLocation`))) (.rotation (`self.GetTransform`)) (.scale (`self.GetTransform`))) "Undefined" "OverrideRootScale" null null)))

(event `Key|LeftMouseButton`
  (params (Key :type "Key Structure"))
  (:`Released`
    (`|ExecutionSequence`
      (:`then_0`
        (`/Engine/EditorBlueprintResources/ActorMacros.Switch Has Authority`
          (:`Authority`
            (`self.ServerCastFireball`))
          (:`Remote`
            (`self.ClientCastFireball`)))))))

(event `ClientCastFireball`
  ;[1 1 1] Cast Fireball
  (`self.ServerCastFireball`))

(fn `UserConstructionScript`)