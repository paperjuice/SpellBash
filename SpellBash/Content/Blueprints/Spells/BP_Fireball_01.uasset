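; Fireball spell projectile that explodes on walls.
; The construction script sets the ProjectileMovement initial speed from MaxSpeed.
; A blocking Sphere hit on a component tagged "Wall" spawns an explosion particle effect at the impact point and destroys the actor; other hits are ignored.
; The fireball also destroys itself after a short lifetime delay, without an explosion.
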(event `self.ReceiveBeginPlay`
  (`|ExecutionSequence`
    (:`then_0`
      ;[1 1 1] After 5 sec destroy
      (`KismetSystemLibrary.Delay` 5.0)
      (`self.K2_DestroyActor`))))

(event `self.Sphere.OnComponentHit`
  (params (HitComponent :type "PrimitiveComponent Object Reference") (OtherActor :type "Actor Object Reference") (OtherComp :type "PrimitiveComponent Object Reference") (NormalImpulse :type "Vector Structure") (Hit :type "HitResult Structure (by ref)"))
  (bind (_bblockinghit _binitialoverlap _time _distance _location _impactpoint _normal _impactnormal _physmat _hitactor _hitcomponent) (`GameplayStatics.BreakHitResult` Hit))
  (`|ExecutionSequence`
    (:`then_0`
      (if (and _bblockinghit (`ActorComponent.ComponentHasTag` _hitcomponent "Wall"))
        (`GameplayStatics.SpawnEmitterAtLocation` "/Game/FXVarietyPack/Particles/P_ky_explosion.P_ky_explosion" _location)
        (`self.K2_DestroyActor`)))))

(fn `UserConstructionScript`
  (set `ProjectileMovementComponent.InitialSpeed` (`self.MaxSpeed`) (`self.ProjectileMovement`)))