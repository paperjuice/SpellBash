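; MC is a player character with cursor aiming that moves independently of its facing and spawns fireballs.
; Vertical and Horizontal axes drive movement along directions built from control pitch with zero yaw, while Tick turns the actor's yaw toward the cursor trace hit.
; BeginPlay applies the camera arm length and maximum walk speed.
; Left mouse spawns a Fireball at the actor's transform and prints a debug string.
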(event `InputAxis|Vertical`
  (params (AxisValue :type "Float (single-precision)"))
  ;[1 1 1] Movement Behaviour
  (`self.AddMovementInput` (`KismetMathLibrary.GetForwardVector` (`KismetMathLibrary.MakeRotator` 0.0 (.pitch (`self.GetControlRotation`)))) AxisValue))

(event `InputAxis|Horizontal`
  (params (AxisValue :type "Float (single-precision)"))
  ;[1 1 1] Movement Behaviour
  (`self.AddMovementInput` (`KismetMathLibrary.GetRightVector` (`KismetMathLibrary.MakeRotator` 0.0 (.pitch (`self.GetControlRotation`)))) AxisValue))

(event `self.ReceiveTick`
  (params (DeltaSeconds :type "Float (single-precision)"))
  (`|ExecutionSequence`
    (:`then_0`
      ;[1 1 1] RotateTowards cursor
      (`self.Rotate_Towards_Cursor`))))

(event `self.ReceiveBeginPlay`
  (`|ExecutionSequence`
    (:`then_0`
      (set `SpringArmComponent.TargetArmLength` (`self.Camera_Length`) (`self.CameraLength`)))
    (:`then_1`
      (set `CharacterMovementComponent.MaxWalkSpeed` (`self.Max_Movement_Speed`) (`self.CharacterMovement`)))))

(event `InputAction|LMB`
  (params (Key :type "Key Structure"))
  (:`Pressed`
    (`|SpawnActorFromClass` "/Game/Blueprints/Spells/Fireball/Fireball.Fireball_C" (`self.GetTransform`) "Undefined" "OverrideRootScale" null null)
    (`KismetSystemLibrary.PrintString` "Hello")))

(fn `Rotate_Towards_Cursor`
  (`self.K2_SetActorRotation` (`KismetMathLibrary.MakeRotator` 0.0 0.0 (.yaw (`KismetMathLibrary.FindLookAtRotation` (`self.K2_GetActorLocation`) (`.Location` (`GameplayStatics.BreakHitResult` (`PlayerController.GetHitResultUnderCursorByChannel` (`GameplayStatics.GetPlayerController` 0) "TraceTypeQuery3" false))))))))

(fn `UserConstructionScript`)